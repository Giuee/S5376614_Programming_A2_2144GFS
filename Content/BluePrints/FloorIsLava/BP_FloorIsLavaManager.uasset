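; Manager for a floor-is-lava puzzle that opens a target door once enough safe tiles have been stepped on.
; On BeginPlay it spawns a grid of BP_FloorTiles offset from its location, passes itself to each, randomly marks each safe or unsafe and counts the safe ones.
; StepOnGoodTile increments a step counter and calls OpenDoor on TargetDoor when it equals the safe tile count.
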(event EventBeginPlay
  (for _index (range 0 3)
    (Variables|Default|SetCurrentX (+ (Variables|Default|GetCurrentX) 2e+02))
    (Variables|Default|SetCurrentY 0.0)
    (for _index_2 (range 0 6)
      (Variables|Default|SetCurrentY (+ (Variables|Default|GetCurrentY) 2e+02))
      (bind _returnvalue (Game|SpawnActorfromClass "/Game/BluePrints/FloorIsLava/BP_FloorTiles.BP_FloorTiles_C" (Math|Transform|MakeTransform (+ (Transformation|GetActorLocation) (Math|Vector|MakeVector (Variables|Default|GetCurrentX) (Variables|Default|GetCurrentY) 0.0))) "Undefined" "MultiplyWithRoot" 0 self 0))
      (Utilities|Array|Add (Variables|Default|GetTileArray) 0)
      (Variables|/Game/BluePrints/FloorIsLava/BP_FloorTiles.BP_FloorTiles_C|SetIsSafe _returnvalue (Utilities|Select :Index (Math|Random|RandomIntegerinRange 0 1) :Option%200 true :Option%201 false))
      (if (Variables|/Game/BluePrints/FloorIsLava/BP_FloorTiles.BP_FloorTiles_C|GetIsSafe _returnvalue)
        (Math|Integer|IncrementInt (Variables|Default|GetAmountofGoodTiles)))))
  (Development|PrintString (Utilities|String|ToString(Integer) (Variables|Default|GetAmountofGoodTiles))))

(event Collision|EventActorBeginOverlap
  (params (OtherActor :type Actor%20Object%20Reference)))

(event EventTick
  (params (DeltaSeconds :type Float%20%28single-precision%29)))

(fn ConstructionScript)

(fn SteponGoodTile
  (bind _result (Math|Integer|IncrementInt (Variables|Default|GetTilesSteppedOn))
    (:%20%20
      (if (== (Variables|Default|GetAmountofGoodTiles) _result)
        (Default|OpenDoor (Variables|Default|GetTargetDoor))))))