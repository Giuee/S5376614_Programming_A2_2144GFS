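; A single tile in a floor-is-lava minigame that is either safe or lava, set by its IsSafe flag.
; The first overlap by the first-person character reveals it, gated by a DoOnce that is never reset.
; Safe tiles change material and notify FloorLavaManager, while lava tiles play a wrong sound, turn to lava and teleport the player to a fixed location.
; ShowFlash offers a safe-flash material that this Blueprint never triggers itself.
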(event EventBeginPlay)

(event Collision|EventActorBeginOverlap
  (params (OtherActor :type Actor%20Object%20Reference))
  (Utilities|Casting|CastToBP_FirstPersonCharacter OtherActor)
  (Utilities|FlowControl|DoOnce false
    (:Completed
      (if (Variables|Default|GetIsSafe)
        (Development|PrintString "Safe")
        (CallFunction|ShowSafe)
        (Default|SteponGoodTile (Variables|Default|GetFloorLavaManager))
        (else
          (Development|PrintString "Lava")
          (Audio|PlaySoundatLocation "/Game/BluePrints/SimonSays/SFX_WRONG.SFX_WRONG" (Transformation|GetActorLocation) "0, 0, 0" 1.0 1.0 0.0 0 0 0 0)
          (Transformation|SetActorLocation (Game|GetPlayerCharacter 0) "2450.000000,2050.000000,10.000000" false false)
          (Rendering|Material|SetMaterial (Variables|Default|GetTiles) 0 "/Game/BluePrints/FloorIsLava/M_Lava.M_Lava"))))))

(event EventTick
  (params (DeltaSeconds :type Float%20%28single-precision%29)))

(fn ConstructionScript)

(fn ShowFlash
  (Rendering|Material|SetMaterial (Variables|Default|GetTiles) 0 "/Game/BluePrints/FloorIsLava/M_SafeFlash.M_SafeFlash"))

(fn ShowSafe
  (Rendering|Material|SetMaterial (Variables|Default|GetTiles) 0 "/Game/BluePrints/FloorIsLava/M_Safe.M_Safe"))