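; Simon Says sequence actor that shows the player a random series of colours by flashing materials on a display mesh.
; BeginPlay fills the sequence with random picks from a materials array, with a length that grows by two per round.
; FlashColour steps through it with a delayed, self-re-entering DoN loop, returning to the wall material between flashes.
; SetColour maps an index to a colour material but is not called here.
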(event Custom|FlashColour
  ;[1 1 1] VERY FIRST FLASH ON RESET IS A BAIT
  (Utilities|FlowControl|Sequence
    (:then_0
      (bind _counter (Utilities|FlowControl|DoN (Utilities|Array|Length (Variables|Default|GetSequence)) :!label _label)
        (:Exit
          (Rendering|Material|SetMaterial (Variables|Default|GetSimonColourStaticMesh) 0 (Utilities|Array|Get(acopy) (Variables|Default|GetSequence) (- _counter 1)))
          (Utilities|FlowControl|Delay 0.5)
          (Rendering|Material|SetMaterial (Variables|Default|GetSimonColourStaticMesh) 0 "/Game/StarterContent/Materials/M_Basic_Wall.M_Basic_Wall")
          (Utilities|FlowControl|Delay 0.1)
          (goto _label))))
    (:then_1
      (goto _label Reset))))

(event EventBeginPlay
  ;[1 1 1] VERY FIRST FLASH ON RESET IS A BAIT
  (CallFunction|SequenceGenerate))

(event Collision|EventActorBeginOverlap
  (params (OtherActor :type Actor%20Object%20Reference)))

(fn ConstructionScript)

(fn SetColour
  (params (ColourIndex :type Integer))
  ;[1 1 1] Switches Colour
  (switch int ColourIndex
    (:0
      (Rendering|Material|SetMaterial (Variables|Default|GetSimonColourStaticMesh) 0 "/Game/BluePrints/SimonSays/m_simoncolourRED.m_simoncolourRED"))
    (:1
      (Rendering|Material|SetMaterial (Variables|Default|GetSimonColourStaticMesh) 0 "/Game/LevelPrototyping/Materials/MI_Solid_Blue.MI_Solid_Blue"))
    (:2
      (Rendering|Material|SetMaterial (Variables|Default|GetSimonColourStaticMesh) 0 "/Game/BluePrints/SimonSays/m_simoncolourYellow.m_simoncolourYellow"))
    (:3
      (Rendering|Material|SetMaterial (Variables|Default|GetSimonColourStaticMesh) 0 "/Game/BluePrints/SimonSays/m_simoncolourGreen.m_simoncolourGreen"))))

(fn SequenceGenerate
  (Utilities|Array|Clear (Variables|Default|GetSequence))
  (bind _length (CallFunction|GetSequenceLength))
  (for _index (range 0 _length)
    (Utilities|Array|Add (Variables|Default|GetSequence) (Utilities|Array|Get(acopy) (Variables|Default|GetMaterials) (Math|Random|RandomIntegerinRange 0 3)))))

(fn GetSequenceLength
  ;[1 1 1] adds 2 colours to the sequence per round
  (return (+ (* (- (Variables|Default|GetCurrentRound) -1) 2) 3)))