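; Simon Says input checker that compares clicks on its four coloured components against the generated sequence and opens a target door once the final round is solved.
; Each click passes its colour material to CheckInput, which steps through the Sequence on BP_SimonSaysSequence.
; Completing a round updates BP_CurrentRoundIndicator and flashes a new sequence.
; A wrong guess plays an error sound and restarts the current round with a fresh sequence.
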(event OnClicked(Yellow)
  (params (TouchedComponent :type Primitive%20Component%20Object%20Reference) (ButtonPressed :type Key%20Structure :default "None"))
  (CallFunction|CheckInput "/Game/BluePrints/SimonSays/m_simoncolourYellow.m_simoncolourYellow"))

(event OnClicked(Red)
  (params (TouchedComponent :type Primitive%20Component%20Object%20Reference) (ButtonPressed :type Key%20Structure :default "None"))
  (CallFunction|CheckInput "/Game/BluePrints/SimonSays/m_simoncolourRED.m_simoncolourRED"))

(event OnClicked(Blue)
  (params (TouchedComponent :type Primitive%20Component%20Object%20Reference) (ButtonPressed :type Key%20Structure :default "None"))
  (CallFunction|CheckInput "/Game/BluePrints/SimonSays/m_simoncolourBlue.m_simoncolourBlue"))

(event OnClicked(Green)
  (params (TouchedComponent :type Primitive%20Component%20Object%20Reference) (ButtonPressed :type Key%20Structure :default "None"))
  (CallFunction|CheckInput "/Game/BluePrints/SimonSays/m_simoncolourGreen.m_simoncolourGreen"))

(event Custom|CheckInput
  (params (CheckValue :type Material%20Object%20Reference))
  (bind _returnvalue (Actor|GetActorOfClass "/Game/BluePrints/SimonSays/BP_SimonSaysSequence.BP_SimonSaysSequence_C"))
  (if (== (Utilities|Array|Get(acopy) (Variables|/Game/BluePrints/SimonSays/BP_SimonSaysSequence.BP_SimonSaysSequence_C|GetSequence _returnvalue) (Variables|Default|GetCheckCurrentGuess)) CheckValue)
    (Math|Integer|IncrementInt (Variables|Default|GetCheckCurrentGuess)
      (:%20%20
        (if (== (Variables|Default|GetCheckCurrentGuess) (Utilities|Array|Length (Variables|/Game/BluePrints/SimonSays/BP_SimonSaysSequence.BP_SimonSaysSequence_C|GetSequence _returnvalue)))
          (if (>= (Variables|Default|GetCurrentRound) 3)
            (Development|PrintString "Puzzle Complete")
            (Default|OpenDoor (Variables|Default|GetTargetDoor))
            (else
              (bind _returnvalue_2 (Actor|GetActorOfClass "/Game/BluePrints/SimonSays/BP_CurrentRoundIndicator.BP_CurrentRoundIndicator_C"))
              (Default|RoundComplete _returnvalue_2 (Variables|Default|GetCurrentRound))
              (Variables|Default|SetCheckCurrentGuess 0)
              (Math|Integer|IncrementInt (Variables|Default|GetCurrentRound)
                (:%20%20
                  (Development|PrintString "next round")
                  (Default|SequenceGenerate _returnvalue)
                  (Default|FlashColour _returnvalue)))))
          (else
            (Development|PrintString "Corect")))))
    (else
      (Audio|PlaySoundatLocation "/Game/BluePrints/SimonSays/SFX_WRONG.SFX_WRONG" (Transformation|GetActorLocation) "0, 0, 0" 1.0 1.0 0.0 0 0 0 0)
      (Default|SequenceGenerate _returnvalue)
      (Default|FlashColour _returnvalue)
      (Variables|Default|SetCheckCurrentGuess 0)
      (Development|PrintString "Reset"))))

(event EventBeginPlay)

(fn ConstructionScript)