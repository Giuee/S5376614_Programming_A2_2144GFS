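; BP_PickupBox is an interactable physics box that the player can pick up.
; On Interact it registers itself as the HoldObject on the first-person player character, then turns off physics simulation on its Box component.
; It does no attaching or movement itself, and it prints debug strings along the way.
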(event EventBeginPlay)

(event Collision|EventActorBeginOverlap
  (params (OtherActor :type Actor%20Object%20Reference)))

(event EventTick
  (params (DeltaSeconds :type Float%20%28single-precision%29)))

(event EventInteract
  (bind _asbp_first_person_character (Utilities|Casting|CastToBP_FirstPersonCharacter (Game|GetPlayerCharacter 0)))
  (bind _output_get (Variables|/Game/FirstPerson/Blueprints/BP_FirstPersonCharacter.BP_FirstPersonCharacter_C|SetHoldObject _asbp_first_person_character self))
  (Development|PrintString "Interact fired")
  (if (Utilities|IsValid _output_get)
    (Development|PrintString "Valid")
    (Physics|SetSimulatePhysics (Variables|Default|GetBox) false)
    (else
      (Development|PrintString "No Valid"))))

(fn ConstructionScript)